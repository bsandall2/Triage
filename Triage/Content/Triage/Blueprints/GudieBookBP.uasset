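; Interactable guide book actor that opens and closes a guide book UI when the player interacts with it.
; Interact fires OpenGuideBook, whose FlipFlop alternates between opening and closing.
; Opening hides the book, spawns a GuideBookWidget and shows the cursor with Game and UI input.
; Closing unhides the book, removes the widget and restores game-only input.
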(event `OpenGuideBook`
  (bind _returnvalue (`GameplayStatics.GetPlayerController` 0))
  (bind _returnvalue_2 (`ActorComponent.GetOwner` (`self.StaticMesh`)))
  (`/Engine/EditorBlueprintResources/StandardMacros.FlipFlop`
    (:`A`
      (`self.SetActorHiddenInGame` _returnvalue_2 true)
      (bind _returnvalue_3 (`|CreateWidget` "/Game/Triage/Widgets/GuideBookWidget.GuideBookWidget_C"))
      (bind _output_get (set `self.GBWidget` _returnvalue_3))
      (`UserWidget.AddToViewport` _output_get 0)
      (`WidgetBlueprintLibrary.SetInputMode_GameAndUIEx` _returnvalue null "DoNotLock" false)
      (set `PlayerController.bShowMouseCursor` true _returnvalue))
    (:`B`
      (`self.SetActorHiddenInGame` _returnvalue_2 false)
      (`Widget.RemoveFromParent` (`self.GBWidget`))
      (`WidgetBlueprintLibrary.SetInputMode_GameOnly` _returnvalue)
      (set `PlayerController.bShowMouseCursor` false _returnvalue))))

(fn `Interact`
  (returns (`Did Interact?` :type Boolean))
  (`self.OpenGuideBook`)
  (return false))

(fn `UserConstructionScript`)