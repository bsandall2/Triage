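; PatientDetailsBP is an interactable that lets the player inspect a patient's details sheet in the Triage game.
; Interact calls InspectPaper, where a FlipFlop alternates between opening and closing the view.
; Opening hides the PatientSheet's owner actor, adds a newly created PatientDetailsWidget to the viewport and enables cursor and UI input.
; Closing unhides that actor, removes the widget and restores game-only input.
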(event `InspectPaper`
  (bind _returnvalue (`GameplayStatics.GetPlayerController` 0))
  (bind _returnvalue_2 (`ActorComponent.GetOwner` (`self.PatientSheet`)))
  (`/Engine/EditorBlueprintResources/StandardMacros.FlipFlop`
    (:`A`
      (`self.SetActorHiddenInGame` _returnvalue_2 true)
      (bind _returnvalue_3 (`|CreateWidget` "/Game/Triage/Widgets/PatientDetailsWidget.PatientDetailsWidget_C"))
      (bind _output_get (set `self.PatientWidget` _returnvalue_3))
      (`UserWidget.AddToViewport` _output_get 0)
      (`WidgetBlueprintLibrary.SetInputMode_GameAndUIEx` _returnvalue _output_get "DoNotLock" false)
      (set `PlayerController.bShowMouseCursor` true _returnvalue))
    (:`B`
      (`self.SetActorHiddenInGame` _returnvalue_2 false)
      (`Widget.RemoveFromParent` (`self.PatientWidget`))
      (`WidgetBlueprintLibrary.SetInputMode_GameOnly` _returnvalue)
      (set `PlayerController.bShowMouseCursor` false _returnvalue))))

(fn `Interact`
  (returns (`Did Interact?` :type Boolean))
  (`self.InspectPaper`)
  (return false))

(fn `UserConstructionScript`)