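; First-person player pawn that handles mouse look, interaction and physics pickup of objects.
; On Interact, a short camera trace calls InteractMessage on InteractInterface actors, or grabs sufficiently light components with a PhysicsHandle until release.
; Look input moves the held object's target in front of the camera.
; Tick repeats the trace to outline interactable static meshes via custom depth stencil, clearing the outline otherwise.
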(event `InputAxis|Mouse Look Left/Right`
  (params (AxisValue :type "Float (single-precision)"))
  (bind _fpp (`self.FPP`))
  ;[1 1 1] Looking Around Controls
  (`self.AddControllerYawInput` AxisValue)
  (`PhysicsHandleComponent.SetTargetLocation` (`self.PhysicsHandle`) (+ (`SceneComponent.K2_GetComponentLocation` _fpp) (* (`SceneComponent.GetForwardVector` _fpp) 100))))

(event `InputAxis|Mouse Look Up/Down`
  (params (AxisValue :type "Float (single-precision)"))
  (bind _fpp (`self.FPP`))
  ;[1 1 1] Looking Around Controls
  (`self.AddControllerPitchInput` AxisValue)
  (`PhysicsHandleComponent.SetTargetLocation` (`self.PhysicsHandle`) (+ (`SceneComponent.K2_GetComponentLocation` _fpp) (* (`SceneComponent.GetForwardVector` _fpp) 100))))

(event `InputAction|Interact`
  (params (Key :type "Key Structure"))
  (bind _fpp (`self.FPP`))
  (bind _returnvalue (`SceneComponent.K2_GetComponentLocation` _fpp))
  ;[1 1 1] Interaction with objects
  (:`Pressed`
    (bind (_outhit _returnvalue_2) (`KismetSystemLibrary.LineTraceSingle` _returnvalue (+ _returnvalue (* (`SceneComponent.GetForwardVector` _fpp) 400)) "TraceTypeQuery1"))
    (if _returnvalue_2
      (bind (_bblockinghit _binitialoverlap _time _distance _location _impactpoint _normal _impactnormal _physmat _hitactor _hitcomponent) (`GameplayStatics.BreakHitResult` _outhit))
      (if (`KismetSystemLibrary.DoesImplementInterface` _hitactor "/Game/Triage/Blueprints/InteractInterface.InteractInterface_C")
        (message `/Game/Triage/Blueprints/InteractInterface.Interact` _hitactor)
        (`KismetSystemLibrary.PrintString` "Interacted" true true (struct :`R` 1.0 :`B` 0.11183 :`A` 1.0))
        (elif (< (`PrimitiveComponent.GetMass` _hitcomponent) 300.0)
          (`PhysicsHandleComponent.GrabComponentAtLocation` (`self.PhysicsHandle`) _hitcomponent "None" _impactpoint)
          (`KismetSystemLibrary.PrintString` "PickedUp" true true (struct :`G` 0.326054 :`B` 1.0 :`A` 1.0))))))
  (:`Released`
    (`PhysicsHandleComponent.ReleaseComponent` (`self.PhysicsHandle`))))

(event `self.ReceiveTick`
  (params (DeltaSeconds :type "Float (single-precision)"))
  (bind _fpp (`self.FPP`))
  (bind _is_outlined_object (`self.Is Outlined Object`))
  (bind _returnvalue (`SceneComponent.K2_GetComponentLocation` _fpp))
  ;[1 1 1] Interaction with objects
  (set `self.Hit Component` false)
  (bind (_outhit _returnvalue_2) (`KismetSystemLibrary.LineTraceSingle` _returnvalue (+ _returnvalue (* (`SceneComponent.GetForwardVector` _fpp) 400)) "TraceTypeQuery1"))
  (if _returnvalue_2
    (bind (_bblockinghit _binitialoverlap _time _distance _location _impactpoint _normal _impactnormal _physmat _hitactor _hitcomponent) (`GameplayStatics.BreakHitResult` _outhit))
    (bind _asstatic_mesh_component (cast `StaticMeshComponent` _hitcomponent)
      (:`then`
        (if (not (== _is_outlined_object _asstatic_mesh_component))
          (`/Engine/EditorBlueprintResources/StandardMacros.IsValid` _is_outlined_object
            (:`Is Valid`
              (`PrimitiveComponent.SetRenderCustomDepth` _is_outlined_object false)
              (`PrimitiveComponent.SetCustomDepthStencilValue` _is_outlined_object 0))
            (:`Is Not Valid`
              _)))
        (set `self.Is Outlined Object` _asstatic_mesh_component)
        (if (`KismetSystemLibrary.DoesImplementInterface` _hitactor "/Game/Triage/Blueprints/InteractInterface.InteractInterface_C")
          (`PrimitiveComponent.SetRenderCustomDepth` _is_outlined_object true)
          (`PrimitiveComponent.SetCustomDepthStencilValue` _is_outlined_object 2)
          (else
            (`/Engine/EditorBlueprintResources/StandardMacros.IsValid` _is_outlined_object :!label _label
              (:`Is Valid`
                (`PrimitiveComponent.SetRenderCustomDepth` _is_outlined_object false)
                (`PrimitiveComponent.SetCustomDepthStencilValue` _is_outlined_object 0)
                (set `self.Is Outlined Object` null))))))
      (:`CastFailed`
        (goto _label)))
    (else
      (goto _label))))

(fn `Interact`
  (returns (`Did Interact?` :type Boolean))
  (return false))

(fn `UserConstructionScript`)