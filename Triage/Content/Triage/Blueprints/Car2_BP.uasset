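; Car actor that drives itself along the spline of a Car2Spline_BP actor in the level.
; On BeginPlay it finds that spline actor and starts a timeline whose play rate is scaled so the trip lasts TimeToComplete.
; Each update maps the timeline alpha to a distance along the spline and sets the car's world location and rotation from that point.
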(event `self.ReceiveBeginPlay`
  (bind _returnvalue (`GameplayStatics.GetActorOfClass` "/Game/Triage/Blueprints/Car2Spline_BP.Car2Spline_BP_C"))
  (set `self.Spline2REF` _returnvalue)
  (`self.MoveCar`))

(event `MoveCar`
  (bind _carspline (`/Game/Triage/Blueprints/Car2Spline_BP.CarSpline` (`self.Spline2REF`)))
  (`TimelineComponent.SetPlayRate` (`self.MoveCarTimeline`) (/ 1.0 (`self.TimeToComplete`)))
  (bind (_direction _movetrack) (`Timeline|MoveCarTimeline`)
    (:`Update`
      (bind _returnvalue (`KismetMathLibrary.Lerp` 0.0 (`SplineComponent.GetSplineLength` (`/Game/Triage/Blueprints/Car2Spline_BP.CarSpline` (`self.Spline2REF`))) _movetrack))
      (`self.K2_SetActorTransform` (`KismetMathLibrary.MakeTransform` (`SplineComponent.GetLocationAtDistanceAlongSpline` _carspline _returnvalue "World") (`SplineComponent.GetRotationAtDistanceAlongSpline` _carspline _returnvalue "World"))))))

(fn `UserConstructionScript`)