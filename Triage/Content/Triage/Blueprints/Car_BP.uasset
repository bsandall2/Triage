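; Car actor that drives itself along the spline of a CarSpline_BP actor in the level.
; On BeginPlay it finds that spline actor by class and starts a timeline with play rate set to 1 / TimeToComplete.
; Each update maps the timeline's MoveTrack alpha to a distance along the spline and sets the car's transform there, using world-space location but local-space rotation.
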(event `self.ReceiveBeginPlay`
  (bind _returnvalue (`GameplayStatics.GetActorOfClass` "/Game/Triage/Blueprints/CarSpline_BP.CarSpline_BP_C"))
  (set `self.SplineREF` _returnvalue)
  (`self.MoveCar`))

(event `MoveCar`
  (bind _carspline (`/Game/Triage/Blueprints/CarSpline_BP.CarSpline` (`self.SplineREF`)))
  (`TimelineComponent.SetPlayRate` (`self.MoveCarTimeline`) (/ 1.0 (`self.TimeToComplete`)))
  (bind (_direction _movetrack) (`Timeline|MoveCarTimeline`)
    (:`Update`
      (bind _returnvalue (`KismetMathLibrary.Lerp` 0.0 (`SplineComponent.GetSplineLength` (`/Game/Triage/Blueprints/CarSpline_BP.CarSpline` (`self.SplineREF`))) _movetrack))
      (`self.K2_SetActorTransform` (`KismetMathLibrary.MakeTransform` (`SplineComponent.GetLocationAtDistanceAlongSpline` _carspline _returnvalue "World") (`SplineComponent.GetRotationAtDistanceAlongSpline` _carspline _returnvalue "Local"))))))

(fn `UserConstructionScript`)