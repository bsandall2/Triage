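; PatientBP is a patient actor in the Triage game that shows a PatientSheet widget when interacted with.
; It creates the widget at BeginPlay, and Interact calls InspectPatient and returns false.
; A FlipFlop in InspectPatient alternates between showing the sheet with Game and UI input and a visible cursor, and removing it to restore game-only input.
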(event `InspectPatient`
  (bind _returnvalue (`GameplayStatics.GetPlayerController` 0))
  ;[1 1 1] Show Patient Details
  (`/Engine/EditorBlueprintResources/StandardMacros.FlipFlop`
    (:`A`
      (`UserWidget.AddToViewport` (stale `self.ReceiveBeginPlay` _returnvalue) 0)
      (`WidgetBlueprintLibrary.SetInputMode_GameAndUIEx` _returnvalue (stale `self.ReceiveBeginPlay` _returnvalue) "DoNotLock" false)
      (set `PlayerController.bShowMouseCursor` true _returnvalue))
    (:`B`
      (`Widget.RemoveFromParent` (stale `self.ReceiveBeginPlay` _returnvalue))
      (`WidgetBlueprintLibrary.SetInputMode_GameOnly` _returnvalue)
      (set `PlayerController.bShowMouseCursor` false _returnvalue))))

(event `self.ReceiveBeginPlay`
  ;[1 1 1] Show Patient Details
  (bind _returnvalue (`|CreateWidget` (`self.PatientSheet`))))

(fn `Interact`
  (returns (`Did Interact?` :type Boolean))
  (`self.InspectPatient`)
  (return false))

(fn `UserConstructionScript`)